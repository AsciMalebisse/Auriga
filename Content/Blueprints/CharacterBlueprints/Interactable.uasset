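; Interactable lootable object that holds a list of item classes, currently seeded on BeginPlay with a test chest piece and a test sword.
; RemoveLootItem finds the looted item's class in the list, removes it, then scans whether any valid entries remain.
; Once empty, it deactivates and collapses the LootBox in the player character's main UI.
; Tick is empty, and some leftover weapon construction and effect-spec nodes are never executed.
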(event EventBeginPlay
  (bind _items (Variables|Default|GetItems))
  (Utilities|Array|Add _items "/Game/ItemsAndEquipment/Equipment/TestChestPiece.TestChestPiece_C")
  (Utilities|Array|Add _items "/Game/ItemsAndEquipment/TestSword.TestSword_C"))

(event EventTick
  (params (DeltaSeconds :type Float%20%28single-precision%29)))

(event EventRemoveLootItem
  (params (LootItem :type Auriga%20Gameplay%20Effect%20Object%20Reference))
  (bind _items (Variables|Default|GetItems))
  (Utilities|Array|RemoveIndex _items (Utilities|Array|FindItem _items (Utilities|GetClass LootItem)))
  (Variables|Default|SetIsEmpty true)
  (bind _array_element (Utilities|Array|ForEachLoopwithBreak _items)
    (:LoopBody
      (if (not (== _array_element 0))
        (Variables|Default|SetIsEmpty false)))
    (:Completed
      (if (Variables|Default|GetIsEmpty)
        (Components|Activation|Deactivate)
        (bind _asplayer_character (Utilities|Casting|CastToPlayerCharacter (Game|GetPlayerCharacter 0)))
        (Widget|SetVisibility (Variables|/Game/Blueprints/UI_Blueprints/MainUI.MainUI_C|GetLootBox (Variables|/Game/Character/PlayerCharacter/PlayerCharacter.PlayerCharacter_C|GetMainUI _asplayer_character)) "Collapsed")))))